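; Game instance for a hide-and-seek game that hosts, finds and joins multiplayer sessions and opens the lobby and tutorial levels.
; Hosting creates a session, saves room name, password, mode and map to a SaveSessionInfo slot named after the player controller, then opens the map as a listen server.
; Searches store LAN results in AvailableSessions, and setter events hold notification info plus music, audio and mouse settings.
; Save-loading logic is present but disconnected.
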(event `Instance_HostLobby`
  (params (GameMap :type String) (useLan :type Boolean) (RoomName :type Text) (RoomPassword :type Text) (GameMode :type String) (PlayerController :type "PlayerController Object Reference"))
  (bind _returnvalue (`KismetSystemLibrary.GetDisplayName` PlayerController))
  ;[1 1 1] Comment
  (`CreateSessionCallbackProxy.CreateSession` PlayerController 2 useLan
    (:`OnSuccess`
      (`KismetSystemLibrary.PrintString` _returnvalue true true (struct :`G` 0.66 :`B` 1.0 :`A` 1.0) 10.0)
      (bind _returnvalue_2 (`GameplayStatics.CreateSaveGameObject` "/Game/UI/MainMenu/SaveSessionInfo.SaveSessionInfo_C"))
      (bind _output_get (set `self.SaveSessionInfoSubClass` _returnvalue_2))
      (bind _assave_session_info (cast `/Game/UI/MainMenu/SaveSessionInfo` _output_get))
      (set `/Game/UI/MainMenu/SaveSessionInfo.RoomName` RoomName _assave_session_info)
      (set `/Game/UI/MainMenu/SaveSessionInfo.RoomPassword` RoomPassword _assave_session_info)
      (set `/Game/UI/MainMenu/SaveSessionInfo.GameMode` GameMode _assave_session_info)
      (set `/Game/UI/MainMenu/SaveSessionInfo.GameMap` GameMap _assave_session_info)
      (`GameplayStatics.SaveGameToSlot` _output_get _returnvalue)
      (`GameplayStatics.OpenLevel` (`KismetStringLibrary.Conv_StringToName` GameMap) true "listen"))
    (:`OnFailure`
      (`KismetSystemLibrary.PrintString` "fail to create session" true true (struct :`R` 1.0 :`G` 0.043975 :`A` 1.0) 10.0))))

(event `Instance_JoinLobby`
  (params (PlayerController :type "PlayerController Object Reference") (Session :type "BlueprintSessionResult Structure"))
  ;[1 1 1] Comment
  (`JoinSessionCallbackProxy.JoinSession` PlayerController Session
    (:`OnSuccess`
      (`KismetSystemLibrary.PrintString` "Joining"))
    (:`OnFailure`
      (`KismetSystemLibrary.PrintString` "Failed to Join Session"))))

(event `Instance_UpdateAvailableSessions`
  (params (PlayerController :type "PlayerController Object Reference"))
  ;[1 1 1] Comment
  (bind _results (`FindSessionsCallbackProxy.FindSessions` PlayerController 6 true)
    (:`OnSuccess`
      (set `self.AvailableSessions` _results))
    (:`OnFailure`
      (`KismetSystemLibrary.PrintString` "Session search failed" true true (struct :`R` 1.0 :`G` 0.028582 :`A` 1.0)))))

(event `OpenTutorial`
  (params (Level :type Name))
  ;[1 1 1] Open Tutorial Level
  (`GameplayStatics.OpenLevel` Level true "listen"))

(event `OpenLobby`
  ;[1 1 1] Open Lobby Level
  (`GameplayStatics.OpenLevel` "Lobby" true "listen"))

(event `NotifyInfo`
  (params (InfoToNotify :type Text))
  ;[1 1 1] Info to be notified
  (set `self.InfoNotify` InfoToNotify))

(event `Settings`
  (params (music :type "Float (double-precision)") (audio :type "Float (double-precision)") (mouse :type "Float (double-precision)"))
  ;[1 1 1] Settings
  (set `self.musicVolume` music)
  (set `self.audioVolume` audio)
  (set `self.mouseSensitive` mouse))