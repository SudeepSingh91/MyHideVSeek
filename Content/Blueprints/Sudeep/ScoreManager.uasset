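; ScoreManager is an actor Blueprint that tracks the Hider's score and triggers the Hider's win in the CaptureThePoint game mode.
; Its TargetScored event increments Score only on the authority and, when it reaches three, casts the game mode to CaptureThePoint and calls HiderWins.
; A ResetScore event, also authority-only, sets the score back to zero.
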(event `TargetScored`
  ;[1 1 1] Hider Scored
  (`/Engine/EditorBlueprintResources/ActorMacros.Switch Has Authority`
    (:`Authority`
      (set `self.Score` (+ (`self.Score`) 1))
      (if (== (`self.Score`) 3)
        (bind _ascapture_the_point (cast `/Game/GameModes/CaptureThePoint` (`GameplayStatics.GetGameMode`)))
        (`/Game/GameModes/CaptureThePoint.HiderWins` _ascapture_the_point)))))

(event `ResetScore`
  ;[1 1 1] Reset Score
  (`/Engine/EditorBlueprintResources/ActorMacros.Switch Has Authority`
    (:`Authority`
      (set `self.Score` 0))))

(fn `UserConstructionScript`)