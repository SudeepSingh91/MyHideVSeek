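; SeekerSpawnBox is a tutorial trigger volume that brings the practice seeker into play when a Hider first overlaps it.
; With the Hider_Tutorial game mode active, it gathers all Seeker_Prac actors and moves the last one found to SpawnPos's transform.
; It then sets the SeekerSpawn flag, so this happens only once, and calls CallSeekerDispatch.
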(event `self.CollisionComponent.OnComponentBeginOverlap`
  (params (OverlappedComponent :type "PrimitiveComponent Object Reference") (OtherActor :type "Actor Object Reference") (OtherComp :type "PrimitiveComponent Object Reference") (OtherBodyIndex :type Integer) (bFromSweep :type Boolean) (SweepResult :type "HitResult Structure (by ref)"))
  (cast `/Game/HiderBP/Blueprints/Hider` OtherActor)
  (if (not (`self.SeekerSpawn`))
    (cast `/Game/GameModes/Hider_Tutorial` (`GameplayStatics.GetGameMode`))
    (bind _outactors (`GameplayStatics.GetAllActorsOfClass` "/Game/Blueprints/Sudeep/Seeker_Prac.Seeker_Prac_C"))
    (for _array_element _outactors
      _)
    (`self.K2_SetActorTransform` _array_element (`self.GetTransform` (`self.SpawnPos`)) false false)
    (set `self.SeekerSpawn` true)
    (`self.SeekerDispatch`)))

(fn `UserConstructionScript`)