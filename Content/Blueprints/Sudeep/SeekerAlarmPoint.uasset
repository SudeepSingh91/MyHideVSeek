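; Seeker alarm point actor that Seekers arm by staying inside its sphere, so it later sounds when a Hider enters.
; On the authority, the first Seeker in starts a ten-second timer, and each Seeker's player controller shows the remaining countdown.
; Leaving clears that Seeker's countdown, and the timer cancels once no Seekers remain.
; ActivateTimer permanently arms the point, after which Hider overlaps play a reveal sound at its location.
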(event `self.Sphere.OnComponentBeginOverlap`
  (params (OtherActor :type "Actor Object Reference") (OtherComp :type "PrimitiveComponent Object Reference") (OtherBodyIndex :type Integer) (bFromSweep :type Boolean) (SweepResult :type "HitResult Structure (by ref)"))
  (`/Engine/EditorBlueprintResources/ActorMacros.Switch Has Authority`
    (:`Authority`
      (bind _asseeker (cast `/Game/SeekerBP/Blueprints/Seeker` OtherActor)
        (:`then`
          (if (not (`self.TimerActivated`))
            (bind _output_get (set `self.NumOfPlayer` (+ (`self.NumOfPlayer`) 1)))
            (if (== _output_get 1)
              (if (not (`self.IsActivating`))
                (set `self.IsActivating` true)
                (bind _returnvalue (`KismetSystemLibrary.K2_SetTimerDelegate` (`|CreateDelegate` :!event `ActivateTimer`) 10.0))
                (bind _output_get_2 (set `self.TimerHandle` _returnvalue))
                (`self.Show Timer On Player` _asseeker (`KismetSystemLibrary.K2_GetTimerRemainingTimeHandle` _output_get_2) :!label _label))
              (else
                (goto _label)))))
        (:`CastFailed`
          (cast `/Game/HiderBP/Blueprints/Hider` OtherActor)
          (if (`self.TimerActivated`)
            (`self.Play Sound`)))))))

(event `Play Sound`
  (`GameplayStatics.PlaySoundAtLocation` "/Game/Sounds/16_bit_Grenade__Reveal__Cue.16_bit_Grenade__Reveal__Cue" (`self.K2_GetActorLocation`)))

(event `self.ReceiveBeginPlay`)

(event `self.ReceiveActorBeginOverlap`
  (params (OtherActor :type "Actor Object Reference")))

(event `self.ReceiveTick`
  (params (DeltaSeconds :type "Float (single-precision)")))

(event `self.Sphere.OnComponentEndOverlap`
  (params (OtherActor :type "Actor Object Reference") (OtherComp :type "PrimitiveComponent Object Reference") (OtherBodyIndex :type Integer))
  (`/Engine/EditorBlueprintResources/ActorMacros.Switch Has Authority`
    (:`Authority`
      (if (not (`self.TimerActivated`))
        (bind _asseeker (cast `/Game/SeekerBP/Blueprints/Seeker` OtherActor))
        (if (`self.IsActivating`)
          (`self.Show Timer On Player` _asseeker)
          (bind _output_get (set `self.NumOfPlayer` (- (`self.NumOfPlayer`) 1)))
          (if (== _output_get 0)
            (set `self.IsActivating` false)
            (`KismetSystemLibrary.K2_ClearTimerHandle` (`self.TimerHandle`))))))))

(event `ActivateTimer`
  (set `self.TimerActivated` true))

(fn `Show Timer On Player`
  (params (Seeker :type "/Game/SeekerBP/Blueprints/Seeker Object Reference") (Time :type "Float (double-precision)"))
  (bind _asctpplayer_controller (cast `/Game/Blueprints/Daniel/CTP/CTPPlayerController` (`Pawn.GetController` Seeker)))
  (`/Game/Blueprints/Daniel/CTP/CTPPlayerController.StartCountdown` _asctpplayer_controller Time))

(fn `UserConstructionScript`)