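; Goo can actor that gradually refills a Hider's goo while the Hider stands in its Region.
; On the server, overlap starts a looping one-second timer that moves one unit of Content to the Hider, with a slurp sound.
; Leaving stops the drain, and emptying also hides the puddle.
; Content's OnRep shrinks the mesh height to show the remaining goo.
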(event `self.ReceiveBeginPlay`
  (`self.SetSlurpSound`))

(event `MakePuddleInvisible`
  (`SceneComponent.SetVisibility` (`self.Puddle`) false false))

(event `SetSlurpSound`
  (`AudioComponent.SetSound` (`self.SlurpSound`) (`self.SlurpBase`)))

(event `self.Region.OnComponentEndOverlap`
  (params (OverlappedComponent :type "PrimitiveComponent Object Reference") (OtherActor :type "Actor Object Reference") (OtherComp :type "PrimitiveComponent Object Reference") (OtherBodyIndex :type Integer))
  (`/Engine/EditorBlueprintResources/ActorMacros.Switch Has Authority`
    (:`Authority`
      (if (== (`self.Content`) 0)
        _
        (elif (== OtherActor (`self.HiderRef`))
          (`self.StopSlurpSound`)
          (set `self.HiderInRange` false)
          (set `self.HiderRef` null)
          (`KismetSystemLibrary.K2_ClearAndInvalidateTimerHandle` (stale `self.Region.OnComponentBeginOverlap` _returnvalue) :!label _label))))))

(event `self.Region.OnComponentBeginOverlap`
  (params (OverlappedComponent :type "PrimitiveComponent Object Reference") (OtherActor :type "Actor Object Reference") (OtherComp :type "PrimitiveComponent Object Reference") (OtherBodyIndex :type Integer) (bFromSweep :type Boolean) (SweepResult :type "HitResult Structure (by ref)"))
  (`/Engine/EditorBlueprintResources/ActorMacros.Switch Has Authority`
    (:`Authority`
      (if (not (== (`self.Content`) 0))
        (bind _ashider (cast `/Game/HiderBP/Blueprints/Hider` OtherActor))
        (set `self.HiderRef` _ashider)
        (`self.PlaySlurpSound`)
        (if (not (`self.HiderInRange`))
          (set `self.HiderInRange` true)
          (bind _returnvalue (`KismetSystemLibrary.K2_SetTimerDelegate` (delegate `Drain Goo`) 1.0 true)))))))

(event `Drain Goo`
  (bind _output_get (set `self.Content` (- (`self.Content`) 1)))
  (`/Game/HiderBP/Blueprints/Hider.GainGoo` (`self.HiderRef`))
  (if (== _output_get 0)
    (`self.StopSlurpSound`)
    (`self.MakePuddleInvisible`)
    (set `self.HiderInRange` false)
    (goto _label)))

(event `PlaySlurpSound`
  (`AudioComponent.Play` (`self.SlurpSound`) 0.0))

(event `StopSlurpSound`
  (`AudioComponent.Stop` (`self.SlurpSound`)))

(fn `OnRep_Content`
  (`SceneComponent.SetWorldScale3D` (`self.StaticMesh`) (`KismetMathLibrary.MakeVector` 0.4 0.4 (/ (`KismetMathLibrary.Conv_IntToDouble` (`self.Content`)) 20.0))))

(fn `UserConstructionScript`)