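; HiderTrail is a short-lived actor that follows the Hider, presumably as the trail it leaves behind.
; On BeginPlay the authority stores the last Hider found in the level as HiderRef, then destroys the trail after an 18-second delay.
; While that reference is valid, Tick copies the Hider's transform every frame, lowered 80 units on Z.
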(event `self.ReceiveBeginPlay`
  ;[1 1 1] Set Hider Reference and destroy actor after 18 seconds
  (`/Engine/EditorBlueprintResources/ActorMacros.Switch Has Authority`
    (:`Authority`
      (`|ExecutionSequence`
        (:`then_0`
          (bind _outactors (`GameplayStatics.GetAllActorsOfClass` "/Game/HiderBP/Blueprints/Hider.Hider_C"))
          (for _array_element _outactors
            _)
          (set `self.HiderRef` _array_element))
        (:`then_1`
          (`KismetSystemLibrary.Delay` 18.0)
          (`self.K2_DestroyActor`))))))

(event `self.ReceiveTick`
  (params (DeltaSeconds :type "Float (single-precision)"))
  (bind _hiderref (`self.HiderRef`))
  ;[1 1 1] Set position as Hider's
  (if (`KismetSystemLibrary.IsValid` _hiderref)
    (`self.K2_SetActorTransform` (`KismetMathLibrary.MakeTransform` (- (.location (`self.GetTransform` _hiderref)) (0.0 0.0 80.0)) (.rotation (`self.GetTransform` _hiderref)) (.scale (`self.GetTransform` _hiderref))))))

(fn `UserConstructionScript`)