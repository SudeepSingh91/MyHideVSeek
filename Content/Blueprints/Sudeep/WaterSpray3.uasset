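; WaterSpray3 is a water spray hit actor that damages Hiders and bursts on certain level geometry.
; Its trigger overlap runs on the server, spawning a large water drop particle actor and destroying itself on a valid hit.
; TriggerBox, ReplaceableMeshActor and Doors_Rev components tagged DoorFrame block it by setting DidHit.
; Hiders take damage only while that flag is unset; other overlaps are ignored.
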(event `self.OverlapTrigger.OnComponentBeginOverlap`
  (params (OverlappedComponent :type "PrimitiveComponent Object Reference") (OtherActor :type "Actor Object Reference") (OtherComp :type "PrimitiveComponent Object Reference") (OtherBodyIndex :type Integer) (bFromSweep :type Boolean) (SweepResult :type "HitResult Structure (by ref)"))
  (bind _returnvalue (`self.GetTransform`))
  (`/Engine/EditorBlueprintResources/ActorMacros.Switch Has Authority`
    (:`Authority`
      (cast `TriggerBox` OtherActor
        (:`then`
          (set `self.DidHit` true)
          (`|SpawnActorFromClass` "/Game/Blueprints/Sudeep/Water_Drop_LRG_Particles.Water_Drop_LRG_Particles_C" _returnvalue "AlwaysSpawn" "OverrideRootScale")
          (`self.K2_DestroyActor`))
        (:`CastFailed`
          (cast `/Game/Blueprints/Daniel/RandomObjectsRoom/ReplaceableMeshActor` OtherActor
            (:`then`
              (set `self.DidHit` true)
              (`|SpawnActorFromClass` "/Game/Blueprints/Sudeep/Water_Drop_LRG_Particles.Water_Drop_LRG_Particles_C" _returnvalue "AlwaysSpawn" "OverrideRootScale")
              (`self.K2_DestroyActor`))
            (:`CastFailed`
              (bind _ashider (cast `/Game/HiderBP/Blueprints/Hider` OtherActor)
                (:`then`
                  (if (not (`self.DidHit`))
                    (`/Game/HiderBP/Blueprints/Hider.ReceiveDamage` _ashider 1)
                    (`|SpawnActorFromClass` "/Game/Blueprints/Sudeep/Water_Drop_LRG_Particles.Water_Drop_LRG_Particles_C" _returnvalue "AlwaysSpawn" "OverrideRootScale")
                    (`self.K2_DestroyActor`)))
                (:`CastFailed`
                  (bind _asdoors_rev (cast `/Game/Blueprints/Sudeep/Doors_Rev` OtherActor))
                  (for _array_element (`self.GetComponentsByTag` _asdoors_rev "/Script/Engine.StaticMeshComponent" "DoorFrame")
                    (if (== _array_element OtherComp)
                      (set `self.DidHit` true)
                      (`|SpawnActorFromClass` "/Game/Blueprints/Sudeep/Water_Drop_LRG_Particles.Water_Drop_LRG_Particles_C" _returnvalue "AlwaysSpawn" "OverrideRootScale")
                      (`self.K2_DestroyActor`))))))))))))

(fn `UserConstructionScript`)