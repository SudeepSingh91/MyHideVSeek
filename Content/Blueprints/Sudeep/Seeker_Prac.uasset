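; Seeker character for a hide-and-seek style game that can be thrown into a frenzy and shoves movable props.
; Overlapping a sparking Hider starts a ten-second frenzy, during which Tick drifts the capsule by a random horizontal offset re-rolled every second by a looping, never-cleared timer.
; Capsule hits on ReplaceableMeshActors reaching above roughly foot height call MoveMesh, with strength scaled from the Seeker's speed and clamped.
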(event `self.BoxCol.OnComponentBeginOverlap`
  (params (OverlappedComponent :type "PrimitiveComponent Object Reference") (OtherActor :type "Actor Object Reference") (OtherComp :type "PrimitiveComponent Object Reference") (OtherBodyIndex :type Integer) (bFromSweep :type Boolean) (SweepResult :type "HitResult Structure (by ref)"))
  (bind _ashider (cast `/Game/HiderBP/Blueprints/Hider` OtherActor))
  (if (`/Game/HiderBP/Blueprints/Hider.IsSpark` _ashider)
    (`KismetSystemLibrary.K2_SetTimer` null "SetVec" 1.0 true)
    (set `self.IsFrenzy` true)
    (`self.SetFrenzy`)
    (`KismetSystemLibrary.Delay` 10.0)
    (set `self.IsFrenzy` false)
    (`self.StopFrenzy`)))

(event `SetVec`
  (set `self.DelVec` (`KismetMathLibrary.MakeVector` (`KismetMathLibrary.RandomFloatInRange` -5.0 5.0) (`KismetMathLibrary.RandomFloatInRange` -5.0 5.0))))

(event `self.ReceiveTick`
  (params (DeltaSeconds :type "Float (single-precision)"))
  (if (`self.IsFrenzy`)
    (`SceneComponent.K2_AddWorldOffset` (`self.CapsuleComponent`) (`self.DelVec`) false false)))

(event `self.CapsuleComponent.OnComponentHit`
  (params (HitComponent :type "PrimitiveComponent Object Reference") (OtherActor :type "Actor Object Reference") (OtherComp :type "PrimitiveComponent Object Reference") (NormalImpulse :type "Vector Structure") (Hit :type "HitResult Structure (by ref)"))
  (bind _returnvalue (`self.K2_GetActorLocation`))
  (bind _returnvalue_2 (`KismetMathLibrary.FTrunc` (/ (`KismetMathLibrary.VSize` (`self.GetVelocity`)) 50.0)))
  (bind _asreplaceable_mesh_actor (cast `/Game/Blueprints/Daniel/RandomObjectsRoom/ReplaceableMeshActor` OtherActor))
  (if (> (+ (.z (`.Max` (`StaticMeshComponent.GetLocalBounds` (`/Game/Blueprints/Daniel/RandomObjectsRoom/ReplaceableMeshActor.StaticMesh` _asreplaceable_mesh_actor)))) (.z (`self.K2_GetActorLocation` _asreplaceable_mesh_actor))) (- (.z (`self.K2_GetActorLocation`)) 86.0))
    (if (> _returnvalue_2 10)
      (`/Game/Blueprints/Daniel/RandomObjectsRoom/ReplaceableMeshActor.MoveMesh` _asreplaceable_mesh_actor _returnvalue 10)
      (elif (< _returnvalue_2 3)
        (`/Game/Blueprints/Daniel/RandomObjectsRoom/ReplaceableMeshActor.MoveMesh` _asreplaceable_mesh_actor _returnvalue 3)
        (else
          (`/Game/Blueprints/Daniel/RandomObjectsRoom/ReplaceableMeshActor.MoveMesh` _asreplaceable_mesh_actor _returnvalue _returnvalue_2))))))

(fn `UserConstructionScript`)