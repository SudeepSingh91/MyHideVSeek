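; Smoke_Green is a short-lived hazard actor that applies a goo smudge to Seekers who enter its box.
; On authority, a box overlap casts to Seeker and calls SetGooSmudge, guarded by the Seeker's IsSmudge flag.
; The flag is cleared right after the call returns, so it only blocks triggers during that call.
; The server destroys the actor a few seconds after BeginPlay.
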(event `self.Box.OnComponentBeginOverlap`
  (params (OverlappedComponent :type "PrimitiveComponent Object Reference") (OtherActor :type "Actor Object Reference") (OtherComp :type "PrimitiveComponent Object Reference") (OtherBodyIndex :type Integer) (bFromSweep :type Boolean) (SweepResult :type "HitResult Structure (by ref)"))
  ;[1 1 1] Set Goo Smudge On Seeker
  (`/Engine/EditorBlueprintResources/ActorMacros.Switch Has Authority`
    (:`Authority`
      (bind _asseeker (cast `/Game/SeekerBP/Blueprints/Seeker` OtherActor))
      (if (not (`/Game/SeekerBP/Blueprints/Seeker.IsSmudge` _asseeker))
        (set `/Game/SeekerBP/Blueprints/Seeker.IsSmudge` true _asseeker)
        (`/Game/SeekerBP/Blueprints/Seeker.SetGooSmudge` _asseeker)
        (set `/Game/SeekerBP/Blueprints/Seeker.IsSmudge` false _asseeker)))))

(event `self.ReceiveBeginPlay`
  ;[1 1 1] Destroy Self
  (`/Engine/EditorBlueprintResources/ActorMacros.Switch Has Authority`
    (:`Authority`
      (`KismetSystemLibrary.Delay` 5.0)
      (`self.K2_DestroyActor`))))

(fn `UserConstructionScript`)