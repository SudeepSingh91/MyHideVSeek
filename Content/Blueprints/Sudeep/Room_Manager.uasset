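; Room manager Blueprint that randomizes the furnishing of a room's placed objects when play begins, on authority only.
; It gives each RoomObj a random target mesh from MeshArray, removing each pick from the pool.
; Objects whose static mesh is Foyer_Table get a vase ReplaceableMeshActor spawned on top with a random offset, recorded in their ObjOnTop list.
; Events for shuffling object positions exist, but their setup and shuffle calls are disconnected.
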(event `SetupArray`
  (for _array_element (`self.RoomObj`)
    (`KismetArrayLibrary.Array_Add` (`self.RoomVec`) (`self.K2_GetActorLocation` _array_element))))

(event `SetRoomPos`
  (bind _roomvec (`self.RoomVec`))
  (for _index (range (`KismetArrayLibrary.Array_Length` (`self.RoomObj`)))
    (bind _output_get (set `self.IterPos` (`KismetArrayLibrary.Array_Get` _roomvec (`KismetMathLibrary.RandomIntegerInRange` 0 (- (`KismetArrayLibrary.Array_Length` _roomvec) 1)))))
    (`KismetArrayLibrary.Array_RemoveItem` (`self.RoomVec`) _output_get)
    (`self.ReplicatePos` (`KismetArrayLibrary.Array_Get` (`self.RoomObj`) _index) _output_get)))

(event `ReplicatePos`
  (params (Obj :type "/Game/Blueprints/Daniel/RandomObjectsRoom/ReplaceableMeshActor Object Reference") (Pos :type "Vector Structure"))
  (`self.K2_SetActorLocation` Obj Pos false false))

(event `self.ReceiveBeginPlay`
  (bind _returnvalue (`KismetMathLibrary.RandomFloatInRange` 10.0 25.0))
  (bind _returnvalue_2 (`KismetArrayLibrary.Array_Length` (`self.MeshArray`)))
  (`/Engine/EditorBlueprintResources/ActorMacros.Switch Has Authority`
    (:`Authority`
      (if (> _returnvalue_2 0)
        (for _array_element (`self.RoomObj`)
          (bind _output_get (set `self.IterAct` (`KismetMathLibrary.RandomIntegerInRange` 0 (- _returnvalue_2 1))))
          (set `/Game/Blueprints/Daniel/RandomObjectsRoom/ReplaceableMeshActor.TargetMesh` (`KismetArrayLibrary.Array_Get` (`self.MeshArray`) _output_get) _array_element)
          (`KismetArrayLibrary.Array_Remove` (`self.MeshArray`) (`self.IterAct`)))
        (for _array_element_2 (`self.RoomObj`)
          (bind _staticmesh (`/Game/Blueprints/Daniel/RandomObjectsRoom/ReplaceableMeshActor.StaticMesh` _array_element_2))
          (if (== (`StaticMeshComponent.StaticMesh` _staticmesh) "/Game/Geometry/FinalArt/FoyerTable/Foyer_Table.Foyer_Table")
            (bind _returnvalue_3 (`|SpawnActorFromClass` "/Game/Blueprints/Daniel/RandomObjectsRoom/ReplaceableMeshActor.ReplaceableMeshActor_C" (`KismetMathLibrary.MakeTransform` (+ (`KismetMathLibrary.MakeVector` 0.0 0.0 (+ (.z (`.Max` (`StaticMeshComponent.GetLocalBounds` _staticmesh))) 5.0)) (`self.K2_GetActorLocation` _array_element_2) (`KismetMathLibrary.MakeVector` _returnvalue _returnvalue))) "Undefined" "OverrideRootScale"))
            (set `/Game/Blueprints/Daniel/RandomObjectsRoom/ReplaceableMeshActor.TargetMesh` "/Game/Geometry/FinalArt/Vases/vase_med_plants_01.vase_med_plants_01" _returnvalue_3)
            (`self.AddOnTop` _returnvalue_3 _array_element_2)))))))

(event `AddOnTop`
  (params (ObjOnTop :type "/Game/Blueprints/Daniel/RandomObjectsRoom/ReplaceableMeshActor Object Reference") (ObjAtBot :type "/Game/Blueprints/Daniel/RandomObjectsRoom/ReplaceableMeshActor Object Reference"))
  (`KismetArrayLibrary.Array_Add` (`/Game/Blueprints/Daniel/RandomObjectsRoom/ReplaceableMeshActor.ObjOnTop` ObjAtBot) ObjOnTop))

(fn `UserConstructionScript`)