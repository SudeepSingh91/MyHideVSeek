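; Consumable is an ammo pickup actor that refills a player's ability ammo on overlap.
; When its static mesh begins overlapping an actor, it casts to Seeker, then Hider, and checks that character's abilities component.
; If AmmoAvailable is below three, it sets it to three and destroys itself; otherwise it stays in the world.
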(event `self.ReceiveBeginPlay`)

(event `self.StaticMeshComponent.OnComponentBeginOverlap`
  (params (OtherActor :type "Actor Object Reference") (OtherComp :type "PrimitiveComponent Object Reference") (OtherBodyIndex :type Integer) (bFromSweep :type Boolean) (SweepResult :type "HitResult Structure (by ref)"))
  ;[1 1 1] Consume Ammo
  (bind _asseeker (cast `/Game/SeekerBP/Blueprints/Seeker` OtherActor)
    (:`then`
      (bind _seekerabilities (`/Game/SeekerBP/Blueprints/Seeker.SeekerAbilities` _asseeker))
      (if (< (`/Game/Blueprints/Sudeep/SeekerAbilities.Ammo_Available` _seekerabilities) 3)
        (set `/Game/Blueprints/Sudeep/SeekerAbilities.Ammo_Available` 3 _seekerabilities)
        (`self.K2_DestroyActor` :!label _label)))
    (:`CastFailed`
      (bind _ashider (cast `/Game/HiderBP/Blueprints/Hider` OtherActor))
      (bind _hiderabilities (`/Game/HiderBP/Blueprints/Hider.HiderAbilities` _ashider))
      (if (< (`/Game/Blueprints/Sudeep/HiderAbilities.Ammo_Available` _hiderabilities) 3)
        (set `/Game/Blueprints/Sudeep/HiderAbilities.Ammo_Available` 3 _hiderabilities)
        (goto _label)))))

(event `self.ReceiveActorBeginOverlap`
  (params (OtherActor :type "Actor Object Reference")))

(event `self.ReceiveTick`
  (params (DeltaSeconds :type "Float (single-precision)")))

(fn `UserConstructionScript`)