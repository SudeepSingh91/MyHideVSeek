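; HiderBase is the hiders' base actor, which a Seeker can destroy by touching it while a Target is captured.
; On the server, its mesh overlap finds captured Targets and resets their position, clears HasBase on every Hider, destroys the base and resets all ScoreManagers.
; An unconnected chain holds unused logic for counting delivered targets and triggering a hider win through the CaptureThePoint game mode.
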(event `self.StaticMesh.OnComponentBeginOverlap`
  (params (OverlappedComponent :type "PrimitiveComponent Object Reference") (OtherActor :type "Actor Object Reference") (OtherComp :type "PrimitiveComponent Object Reference") (OtherBodyIndex :type Integer) (bFromSweep :type Boolean) (SweepResult :type "HitResult Structure (by ref)"))
  (`/Engine/EditorBlueprintResources/ActorMacros.Switch Has Authority`
    (:`Authority`
      (cast `/Game/SeekerBP/Blueprints/Seeker` OtherActor)
      (bind _outactors (`GameplayStatics.GetAllActorsOfClass` "/Game/Blueprints/Sudeep/Target.Target_C"))
      (for _array_element _outactors
        (if (`/Game/Blueprints/Sudeep/Target.IsCaptured` _array_element)
          (`/Game/Blueprints/Sudeep/Target.ResetPos` _array_element)
          (bind _outactors_2 (`GameplayStatics.GetAllActorsOfClass` "/Game/HiderBP/Blueprints/Hider.Hider_C"))
          (for _array_element_2 _outactors_2
            (set `/Game/HiderBP/Blueprints/Hider.HasBase` false _array_element_2))
          (`self.K2_DestroyActor`)
          (bind _outactors_3 (`GameplayStatics.GetAllActorsOfClass` "/Game/Blueprints/Sudeep/ScoreManager.ScoreManager_C"))
          (for _array_element_3 _outactors_3
            (`/Game/Blueprints/Sudeep/ScoreManager.ResetScore` _array_element_3)))))))

(fn `UserConstructionScript`)