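; Door collider Blueprint whose box overlap reacts to log blockades and to a frenzied Seeker.
; An overlapping Blockade_Logs is destroyed and replaced by a Door_Blocking actor spawned at BlockPos.
; A frenzied Seeker loses frenzy and starts the Punch component sliding every tick, with no stop.
; After a short delay, that Seeker teleports to each HiderBase in turn, ending at the last one.
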(event `self.Box.OnComponentBeginOverlap`
  (params (OverlappedComponent :type "PrimitiveComponent Object Reference") (OtherActor :type "Actor Object Reference") (OtherComp :type "PrimitiveComponent Object Reference") (OtherBodyIndex :type Integer) (bFromSweep :type Boolean) (SweepResult :type "HitResult Structure (by ref)"))
  (bind _blockpos (`self.BlockPos`))
  (bind _asblockade_logs (cast `/Game/Blueprints/Sudeep/Blockade_Logs` OtherActor)
    (:`then`
      (`self.K2_DestroyActor` _asblockade_logs)
      (`|SpawnActorFromClass` "/Game/Blueprints/Sudeep/Door_Blocking.Door_Blocking_C" (`KismetMathLibrary.MakeTransform` (`SceneComponent.K2_GetComponentLocation` _blockpos) (`SceneComponent.K2_GetComponentRotation` _blockpos) (1.0 1.0 1.0)) "Undefined" "OverrideRootScale"))
    (:`CastFailed`
      (bind _asseeker (cast `/Game/SeekerBP/Blueprints/Seeker` OtherActor))
      (if (`/Game/SeekerBP/Blueprints/Seeker.IsFrenzy` _asseeker)
        (set `self.IsPunching` true)
        (set `/Game/SeekerBP/Blueprints/Seeker.IsFrenzy` false _asseeker)
        (`KismetSystemLibrary.Delay` 0.5)
        (bind _outactors (`GameplayStatics.GetAllActorsOfClass` "/Game/Blueprints/Sudeep/HiderBase.HiderBase_C"))
        (for _array_element _outactors
          (`self.K2_SetActorLocation` _asseeker (`self.K2_GetActorLocation` _array_element) false false))))))

(event `self.ReceiveTick`
  (params (DeltaSeconds :type "Float (single-precision)"))
  (if (`self.IsPunching`)
    (`SceneComponent.K2_AddLocalOffset` (`self.Punch`) (0.0 20.0 0.0) false false)))

(fn `UserConstructionScript`)