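; Paint grenade projectile that detects and paints Hiders within a radius of where it hits.
; On component hit, a sphere overlap calls Paint on each Hider found and spawns a paint effect and trail.
; Non-Hider or empty results spawn a smokeless grenade effect instead.
; On authority, it turns off replication on the spawned effects, plays the reveal sound via ReplicateSound and destroys itself.
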(event `ReplicateSound`
  (params (Pos :type "Vector Structure"))
  ;[1 1 1] Hider Detection
  (`GameplayStatics.PlaySoundAtLocation` "/Game/Sounds/16_bit_Grenade__Reveal_.16_bit_Grenade__Reveal_" Pos))

(event `self.StaticMeshComponent.OnComponentHit`
  (params (HitComponent :type "PrimitiveComponent Object Reference") (OtherActor :type "Actor Object Reference") (OtherComp :type "PrimitiveComponent Object Reference") (NormalImpulse :type "Vector Structure") (Hit :type "HitResult Structure (by ref)"))
  (bind (_bblockinghit _binitialoverlap _time _location) (`GameplayStatics.BreakHitResult` Hit))
  (bind _returnvalue (`KismetMathLibrary.MakeTransform` _location (struct) (1.0 1.0 1.0)))
  ;[1 1 1] Hider Detection
  (bind (_outactors _returnvalue_2) (`KismetSystemLibrary.SphereOverlapActors_NEW` _location 300.0 (`|MakeArray` "ObjectTypeQuery2" "ObjectTypeQuery3" :!type "EObjectTypeQuery Enum")))
  (if _returnvalue_2
    (for _array_element _outactors
      (bind _ashider (cast `/Game/HiderBP/Blueprints/Hider` _array_element)
        (:`then`
          (`/Game/HiderBP/Blueprints/Hider.Paint` _ashider)
          (bind _returnvalue_3 (`|SpawnActorFromClass` "/Game/Blueprints/Sudeep/PaintEffect.PaintEffect_C" _returnvalue "AlwaysSpawn" "OverrideRootScale"))
          (bind _returnvalue_4 (`|SpawnActorFromClass` "/Game/Blueprints/Sudeep/HiderTrail.HiderTrail_C" (`self.GetTransform` _ashider) "AlwaysSpawn" "OverrideRootScale"))
          (`/Engine/EditorBlueprintResources/ActorMacros.Switch Has Authority`
            (:`Authority`
              (`self.SetReplicates` _returnvalue_3 false)
              (`self.SetReplicates` _returnvalue_4 false))))
        (:`CastFailed`
          (bind _returnvalue_5 (`|SpawnActorFromClass` "/Game/Blueprints/Sudeep/P_PaintGrenade_NoSmoke.P_PaintGrenade_NoSmoke_C" _returnvalue "AlwaysSpawn" "OverrideRootScale" :!label _label))
          (`/Engine/EditorBlueprintResources/ActorMacros.Switch Has Authority`
            (:`Authority`
              (`self.SetReplicates` _returnvalue_5 false)))))
      (`self.ReplicateSound` _location)
      (`self.Explode`))
    (else
      (goto _label))))

(event `Explode`
  ;[1 1 1] Explode
  (`self.K2_DestroyActor`))

(fn `UserConstructionScript`)