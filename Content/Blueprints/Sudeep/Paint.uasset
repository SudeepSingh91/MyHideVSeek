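; Paint actor that drops straight down until it lands at a fixed floor height or touches a trigger box.
; Tick moves it down by a fixed step per frame, not scaled by delta time or swept, and pins it to the floor height once at or below it.
; The static mesh's begin-overlap with any TriggerBox sets IsColl, which halts the movement and is never cleared here.
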(event `self.ReceiveTick`
  (params (DeltaSeconds :type "Float (single-precision)"))
  (bind _returnvalue (`self.K2_GetActorLocation`))
  (if (`self.IsColl`)
    _
    (elif (> (.z _returnvalue) 3.5)
      (`self.K2_SetActorLocation` (- _returnvalue (0.0 0.0 10.0)))
      (else
        (`self.K2_SetActorLocation` (`KismetMathLibrary.MakeVector` (.x _returnvalue) (.y _returnvalue) 3.5))))))

(event `self.StaticMeshComponent.OnComponentBeginOverlap`
  (params (OverlappedComponent :type "PrimitiveComponent Object Reference") (OtherActor :type "Actor Object Reference") (OtherComp :type "PrimitiveComponent Object Reference") (OtherBodyIndex :type Integer) (bFromSweep :type Boolean) (SweepResult :type "HitResult Structure (by ref)"))
  (cast `TriggerBox` OtherActor)
  (set `self.IsColl` true))

(fn `UserConstructionScript`)