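; Double swing door for Hiders and Seekers that opens away from whoever enters its trigger box and closes when that actor leaves.
; A dot product picks the swing direction, and opening nudges ReplaceableMeshActors on one side via MoveMesh.
; Authority-only Tick rotates both hinges oppositely toward a 90-degree limit, based on the opener's velocity or detected obstacles.
; Box overlap checks delay closing while another player or replaceable mesh occupies the checked side.
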(event `self.Box.OnComponentBeginOverlap`
  (params (OverlappedComponent :type "PrimitiveComponent Object Reference") (OtherActor :type "Actor Object Reference") (OtherComp :type "PrimitiveComponent Object Reference") (OtherBodyIndex :type Integer) (bFromSweep :type Boolean) (SweepResult :type "HitResult Structure (by ref)"))
  (bind _ashider (cast `/Game/HiderBP/Blueprints/Hider` OtherActor)
    (:`then`
      (if (not (`self.DoorOpen`))
        (`self.OpenDoor` _ashider)))
    (:`CastFailed`
      (bind _asseeker (cast `/Game/SeekerBP/Blueprints/Seeker` OtherActor))
      (if (not (`self.DoorOpen`))
        (`self.OpenDoor` _asseeker)))))

(event `DoorRotations`
  (params (Rot :type "Rotator Structure"))
  (`SceneComponent.K2_AddLocalRotation` (`self.LHinge`) Rot false false)
  (`SceneComponent.K2_AddLocalRotation` (`self.RHinge`) (* Rot -1) false false))

(event `self.Box.OnComponentEndOverlap`
  (params (OverlappedComponent :type "PrimitiveComponent Object Reference") (OtherActor :type "Actor Object Reference") (OtherComp :type "PrimitiveComponent Object Reference") (OtherBodyIndex :type Integer))
  (if (== OtherActor (`self.ObjInDoor`))
    (`self.CloseDoor`)))

(event `self.ReceiveTick`
  (params (DeltaSeconds :type "Float (single-precision)"))
  (`/Engine/EditorBlueprintResources/ActorMacros.Switch Has Authority`
    (:`Authority`
      (set `self.deltaTimer` DeltaSeconds)
      (if (`self.DoorOpen`)
        (bind _isthere (`self.CheckForObjects`))
        (if _isthere
          (`self.ControlRotation`)
          (else
            (bind _iscor (`self.ConfirmDir`))
            (if _iscor
              (`self.ControlRotation`))))
        (elif (!= (`self.RotLimit`) 0.0)
          (bind _isthere_2 (`self.CheckForObjects`))
          (if _isthere_2
            _
            (elif (> (`self.RotLimit`) 0.0)
              (`self.DoorRotations` (* (`KismetMathLibrary.MakeRotator` 0.0 0.0 (* -5.0 65.0)) (`self.deltaTimer`)))
              (set `self.RotLimit` (- (`self.RotLimit`) (* (* 5.0 65.0) (`self.deltaTimer`))))
              (else
                (`self.DoorRotations` (* (`KismetMathLibrary.MakeRotator` 0.0 0.0 (* 5.0 65.0)) (`self.deltaTimer`)))
                (set `self.RotLimit` (+ (`self.RotLimit`) (* (* 5.0 65.0) (`self.deltaTimer`))))))))))))

(event `ControlRotation`
  (if (`self.OpenFront`)
    (if (< (`self.RotLimit`) 90.0)
      (`self.DoorRotations` (* (`KismetMathLibrary.MakeRotator` 0.0 0.0 (* 5.0 65.0)) (`self.deltaTimer`)))
      (set `self.RotLimit` (+ (`self.RotLimit`) (* (* 5.0 65.0) (`self.deltaTimer`)))))
    (elif (> (`self.RotLimit`) -90.0)
      (`self.DoorRotations` (* (`KismetMathLibrary.MakeRotator` 0.0 0.0 (* -5.0 65.0)) (`self.deltaTimer`)))
      (set `self.RotLimit` (- (`self.RotLimit`) (* (* 5.0 65.0) (`self.deltaTimer`)))))))

(event `CloseDoor`
  (set `self.DoorOpen` false))

(event `OpenDoor`
  (params (Obj :type "Actor Object Reference"))
  (set `self.ObjInDoor` Obj)
  (set `self.DoorOpen` true)
  (`self.CheckDir`)
  (`self.PushObjectsAhead`))

(fn `CheckDir`
  (if (> (`KismetMathLibrary.Dot_VectorVector` (- (`self.K2_GetActorLocation` (`self.ObjInDoor`)) (`self.K2_GetActorLocation`)) (`self.GetActorRightVector`)) 0.0)
    (set `self.OpenFront` false)
    (else
      (set `self.OpenFront` true))))

(fn `CheckForObjects`
  (returns (IsThere :type Boolean))
  (bind _rotlimit (`self.RotLimit`))
  (set `self.FoundSecondObj` false)
  (if (!= _rotlimit 0.0)
    (if (> _rotlimit 0.0)
      (bind _outactors (`KismetSystemLibrary.BoxOverlapActors_NEW` (`SceneComponent.K2_GetComponentLocation` (`self.FRay`)) (120.0 60.0 180.0) (`|MakeArray` "ObjectTypeQuery2" :!type "EObjectTypeQuery Enum") null (`|MakeArray` self (`self.ObjInDoor`) :!type "Actor Object Reference")))
      (for _array_element _outactors
        (if (!= _array_element (`self.ObjInDoor`))
          (cast `/Game/HiderBP/Blueprints/Hider` _array_element
            (:`then`
              _)
            (:`CastFailed`
              (cast `/Game/SeekerBP/Blueprints/Seeker` _array_element
                (:`then`
                  _)
                (:`CastFailed`
                  (cast `/Game/Blueprints/Daniel/RandomObjectsRoom/ReplaceableMeshActor` _array_element)))))
          (set `self.FoundSecondObj` true)))
      (if (`self.FoundSecondObj`)
        (return true)
        (else
          (return false)))
      (else
        (bind _outactors_2 (`KismetSystemLibrary.BoxOverlapActors_NEW` (`SceneComponent.K2_GetComponentLocation` (`self.BRay`)) (120.0 60.0 180.0) (`|MakeArray` "ObjectTypeQuery2" :!type "EObjectTypeQuery Enum") null (`|MakeArray` self (`self.ObjInDoor`) :!type "Actor Object Reference")))
        (for _array_element_2 _outactors_2
          (if (!= _array_element_2 (`self.ObjInDoor`))
            (cast `/Game/HiderBP/Blueprints/Hider` _array_element_2
              (:`then`
                _)
              (:`CastFailed`
                (cast `/Game/SeekerBP/Blueprints/Seeker` _array_element_2
                  (:`then`
                    _)
                  (:`CastFailed`
                    (cast `/Game/Blueprints/Daniel/RandomObjectsRoom/ReplaceableMeshActor` _array_element_2)))))
            (set `self.FoundSecondObj` true)))
        (if (`self.FoundSecondObj`)
          (return true)
          (else
            (return false)))))
    (else
      (return false))))

(fn `ConfirmDir`
  (returns (IsCor :type Boolean))
  (if (== (`KismetMathLibrary.Dot_VectorVector` (`self.GetVelocity` (`self.ObjInDoor`)) (`self.GetActorRightVector`)) 0.0)
    (return false)
    (elif (`self.OpenFront`)
      (return (> (`KismetMathLibrary.Dot_VectorVector` (`self.GetVelocity` (`self.ObjInDoor`)) (`self.GetActorRightVector`)) 0.0))
      (else
        (return (< (`KismetMathLibrary.Dot_VectorVector` (`self.GetVelocity` (`self.ObjInDoor`)) (`self.GetActorRightVector`)) 0.0))))))

(fn `PushObjectsAhead`
  (bind _returnvalue (`self.K2_GetActorLocation`))
  (if (`self.OpenFront`)
    (bind _outactors (`KismetSystemLibrary.BoxOverlapActors_NEW` (`SceneComponent.K2_GetComponentLocation` (`self.BRay`)) (120.0 60.0 180.0) (`|MakeArray` "ObjectTypeQuery2" :!type "EObjectTypeQuery Enum") null (`|MakeArray` self (`self.ObjInDoor`) :!type "Actor Object Reference")))
    (for _array_element _outactors
      (bind _asreplaceable_mesh_actor (cast `/Game/Blueprints/Daniel/RandomObjectsRoom/ReplaceableMeshActor` _array_element))
      (`/Game/Blueprints/Daniel/RandomObjectsRoom/ReplaceableMeshActor.MoveMesh` _asreplaceable_mesh_actor _returnvalue 3))
    (else
      (bind _outactors_2 (`KismetSystemLibrary.BoxOverlapActors_NEW` (`SceneComponent.K2_GetComponentLocation` (`self.FRay`)) (120.0 60.0 180.0) (`|MakeArray` "ObjectTypeQuery2" :!type "EObjectTypeQuery Enum") null (`|MakeArray` self (`self.ObjInDoor`) :!type "Actor Object Reference")))
      (for _array_element_2 _outactors_2
        (bind _asreplaceable_mesh_actor_2 (cast `/Game/Blueprints/Daniel/RandomObjectsRoom/ReplaceableMeshActor` _array_element_2))
        (`/Game/Blueprints/Daniel/RandomObjectsRoom/ReplaceableMeshActor.MoveMesh` _asreplaceable_mesh_actor_2 _returnvalue 3)))))

(fn `UserConstructionScript`)