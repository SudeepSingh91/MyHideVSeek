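; A non-playable actor that gets briefly pushed horizontally away from a given world position.
; MoveMesh, on the authority only, stores a flattened, scaled direction from that position to the actor and restarts a short timer.
; Authority-side Tick then calls MoveObject each frame for a swept, delta-time-scaled world offset until about 0.2 seconds elapse.
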(event `self.ReceiveTick`
  (params (DeltaSeconds :type "Float (single-precision)"))
  (`/Engine/EditorBlueprintResources/ActorMacros.Switch Has Authority`
    (:`Authority`
      (set `self.deltaTimer` DeltaSeconds)
      (if (`self.Can_Move`)
        (bind _output_get (set `self.timer` (+ (`self.timer`) (`self.deltaTimer`))))
        (if (> _output_get 0.2)
          (set `self.timer` 0.0)
          (set `self.Can_Move` false)
          (else
            (`self.MoveObject` (* (* (`self.MovVec`) 65) (`self.deltaTimer`)))))))))

(event `MoveObject`
  (params (Vec :type "Vector Structure"))
  (`self.K2_AddActorWorldOffset` Vec true))

(fn `MoveMesh`
  (params (DirVec :type "Vector Structure"))
  (`/Engine/EditorBlueprintResources/ActorMacros.Switch Has Authority`
    (:`Authority`
      (set `self.MovVec` (* (`KismetMathLibrary.Normal` (- (`KismetMathLibrary.MakeVector` (.x (`self.K2_GetActorLocation`)) (.y (`self.K2_GetActorLocation`))) (`KismetMathLibrary.MakeVector` (.x DirVec) (.y DirVec)))) 2))
      (set `self.Can_Move` true)
      (set `self.timer` 0.0))))

(fn `UserConstructionScript`)