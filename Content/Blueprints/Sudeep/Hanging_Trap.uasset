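; Hanging trap actor that drops on a Hider who enters its trigger Box.
; The overlap flags the Hider as trapped and starts Tick moving Pivot down by a fixed, unswept, frame-rate-dependent offset.
; Pivot hits call ReceiveDamage with zero on a Hider; any other hit stops the fall and destroys the trigger.
; The Cylinder component turns invisible shortly after play begins.
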(event `self.ReceiveBeginPlay`
  (`KismetSystemLibrary.Delay` 2.0)
  (`SceneComponent.SetVisibility` (`self.Cylinder`) false false))

(event `self.ReceiveTick`
  (params (DeltaSeconds :type "Float (single-precision)"))
  (if (`self.Is_Fall`)
    (`SceneComponent.K2_AddLocalOffset` (`self.Pivot`) (0.0 0.0 -20.0) false false)))

(event `self.Box.OnComponentBeginOverlap`
  (params (OverlappedComponent :type "PrimitiveComponent Object Reference") (OtherActor :type "Actor Object Reference") (OtherComp :type "PrimitiveComponent Object Reference") (OtherBodyIndex :type Integer) (bFromSweep :type Boolean) (SweepResult :type "HitResult Structure (by ref)"))
  (bind _ashider (cast `/Game/HiderBP/Blueprints/Hider` OtherActor))
  (set `/Game/HiderBP/Blueprints/Hider.Is_Trapped` true _ashider)
  (set `self.Is_Fall` true))

(event `self.Pivot.OnComponentHit`
  (params (HitComponent :type "PrimitiveComponent Object Reference") (OtherActor :type "Actor Object Reference") (OtherComp :type "PrimitiveComponent Object Reference") (NormalImpulse :type "Vector Structure") (Hit :type "HitResult Structure (by ref)"))
  (bind _ashider (cast `/Game/HiderBP/Blueprints/Hider` OtherActor)
    (:`then`
      (`/Game/HiderBP/Blueprints/Hider.ReceiveDamage` _ashider 0))
    (:`CastFailed`
      (set `self.Is_Fall` false)
      (`ActorComponent.K2_DestroyComponent` (`self.Box`)))))

(fn `UserConstructionScript`)