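; Double swinging door that Hiders and Seekers push open away from the side they approach.
; Per-leaf overlaps pick direction by dot product, shift a clearance box to the swing side and shove ReplaceableMeshActors inside it.
; Authority-side Tick rotates hinges through Rep events while the player keeps moving in the entry direction, faster for Flash Hiders.
; Leaves ease shut once the player exits the outer box and clearance boxes are empty.
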(event `RepLRot`
  (params (DelRot :type "Rotator Structure"))
  (`SceneComponent.K2_AddLocalRotation` (`self.LHinge`) DelRot false false))

(event `RepRRot`
  (params (DelRot :type "Rotator Structure"))
  (`SceneComponent.K2_AddLocalRotation` (`self.RHinge`) DelRot false false))

(event `RepLBlock`
  (params (DelVec :type "Vector Structure"))
  (`SceneComponent.K2_AddWorldOffset` (`self.LLBox`) DelVec false false))

(event `RepRBlock`
  (params (DelVec :type "Vector Structure"))
  (`SceneComponent.K2_AddWorldOffset` (`self.RLBox`) DelVec false false))

(event `self.Box.OnComponentEndOverlap`
  (params (OverlappedComponent :type "PrimitiveComponent Object Reference") (OtherActor :type "Actor Object Reference") (OtherComp :type "PrimitiveComponent Object Reference") (OtherBodyIndex :type Integer))
  ;[1 1 1] Hider And Seeker Exit
  (`/Engine/EditorBlueprintResources/ActorMacros.Switch Has Authority`
    (:`Authority`
      (if (== OtherActor (`self.Player`))
        (set `self.LeftCheck` true)
        (set `self.RightCheck` true)))))

(event `self.RBox.OnComponentBeginOverlap`
  (params (OverlappedComponent :type "PrimitiveComponent Object Reference") (OtherActor :type "Actor Object Reference") (OtherComp :type "PrimitiveComponent Object Reference") (OtherBodyIndex :type Integer) (bFromSweep :type Boolean) (SweepResult :type "HitResult Structure (by ref)"))
  ;[1 1 1] Decide Direction For Right Door
  (if (not (`self.HitRight`))
    (bind _asseeker (cast `/Game/SeekerBP/Blueprints/Seeker` OtherActor)
      (:`then`
        (set `self.Player` _asseeker)
        (set `self.HitRight` true)
        (bind _dir (`self.CalculateSwingingDir` (`self.K2_GetActorLocation` _asseeker)))
        (set `self.Rdir` _dir))
      (:`CastFailed`
        (bind _ashider (cast `/Game/HiderBP/Blueprints/Hider` OtherActor))
        (set `self.Player` _ashider)
        (set `self.HitRight` true)
        (bind _dir_2 (`self.CalculateSwingingDir` (`self.K2_GetActorLocation` _ashider)))
        (set `self.Rdir` _dir_2)))
    (`self.SetVelocityDir`)
    (set `self.RightCheck` false)
    (`self.MoveRightCollider`)
    (bind _output_get (set `self.RObjArr` (`PrimitiveComponent.GetOverlappingActors` (`self.RLBox`) "/Game/Blueprints/Daniel/RandomObjectsRoom/ReplaceableMeshActor.ReplaceableMeshActor_C")))
    (for _array_element _output_get
      (bind _asreplaceable_mesh_actor (cast `/Game/Blueprints/Daniel/RandomObjectsRoom/ReplaceableMeshActor` _array_element))
      (`/Game/Blueprints/Daniel/RandomObjectsRoom/ReplaceableMeshActor.MoveMesh` _asreplaceable_mesh_actor (`KismetMathLibrary.MakeVector` (.x (`self.K2_GetActorLocation`)) (.y (`self.K2_GetActorLocation`)) 5.0) 6))))

(event `MoveRightCollider`
  ;[1 1 1] Decide Direction For Right Door
  (switch `int` (`self.Rdir`)
    (:`0`
      (`self.RepRBlock` (* (`self.GetActorRightVector`) -30)))
    (:`1`
      (`self.RepRBlock` (* (`self.GetActorRightVector`) 30)))))

(event `ResetLeftCollider`
  ;[1 1 1] Player Exit
  (switch `int` (`self.Ldir`)
    (:`0`
      (`SceneComponent.K2_AddWorldOffset` (`self.LLBox`) (* (`self.GetActorRightVector`) 30) false false))
    (:`1`
      (`SceneComponent.K2_AddWorldOffset` (`self.LLBox`) (* (`self.GetActorRightVector`) -30) false false)))
  (set `self.LeftCheck` false))

(event `CheckSpace`
  ;[1 1 1] Player Exit
  (`/Engine/EditorBlueprintResources/ActorMacros.Switch Has Authority`
    (:`Authority`
      (`|ExecutionSequence`
        (:`then_0`
          (if (`self.HitLeft`)
            (if (`self.LeftCheck`)
              (bind _output_get (set `self.LObjArr` (`PrimitiveComponent.GetOverlappingActors` (`self.LLBox`) "/Game/Blueprints/Daniel/RandomObjectsRoom/ReplaceableMeshActor.ReplaceableMeshActor_C")))
              (if (== (`KismetArrayLibrary.Array_Length` _output_get) 0)
                (set `self.HitLeft` false)
                (`self.ResetLeftCollider`)))))
        (:`then_1`
          (if (`self.HitRight`)
            (if (`self.RightCheck`)
              (bind _output_get_2 (set `self.RObjArr` (`PrimitiveComponent.GetOverlappingActors` (`self.RLBox`) "/Game/Blueprints/Daniel/RandomObjectsRoom/ReplaceableMeshActor.ReplaceableMeshActor_C")))
              (if (== (`KismetArrayLibrary.Array_Length` _output_get_2) 0)
                (set `self.HitRight` false)
                (`self.ResetRightCollider`)))))))))

(event `ResetRightCollider`
  ;[1 1 1] Player Exit
  (switch `int` (`self.Rdir`)
    (:`0`
      (`SceneComponent.K2_AddWorldOffset` (`self.RLBox`) (* (`self.GetActorRightVector`) 30) false false))
    (:`1`
      (`SceneComponent.K2_AddWorldOffset` (`self.RLBox`) (* (`self.GetActorRightVector`) -30) false false)))
  (set `self.RightCheck` false))

(event `self.LBox.OnComponentBeginOverlap`
  (params (OverlappedComponent :type "PrimitiveComponent Object Reference") (OtherActor :type "Actor Object Reference") (OtherComp :type "PrimitiveComponent Object Reference") (OtherBodyIndex :type Integer) (bFromSweep :type Boolean) (SweepResult :type "HitResult Structure (by ref)"))
  ;[1 1 1] Decide Direction For Left Door
  (if (not (`self.HitLeft`))
    (bind _asseeker (cast `/Game/SeekerBP/Blueprints/Seeker` OtherActor)
      (:`then`
        (set `self.Player` _asseeker)
        (set `self.HitLeft` true)
        (bind _dir (`self.CalculateSwingingDir` (`self.K2_GetActorLocation` _asseeker)))
        (set `self.Ldir` _dir))
      (:`CastFailed`
        (bind _ashider (cast `/Game/HiderBP/Blueprints/Hider` OtherActor))
        (set `self.Player` _ashider)
        (set `self.HitLeft` true)
        (bind _dir_2 (`self.CalculateSwingingDir` (`self.K2_GetActorLocation` _ashider)))
        (set `self.Ldir` _dir_2)))
    (`self.SetVelocityDir`)
    (set `self.LeftCheck` false)
    (`self.MoveLeftCollider`)
    (bind _output_get (set `self.LObjArr` (`PrimitiveComponent.GetOverlappingActors` (`self.LLBox`) "/Game/Blueprints/Daniel/RandomObjectsRoom/ReplaceableMeshActor.ReplaceableMeshActor_C")))
    (for _array_element _output_get
      (bind _asreplaceable_mesh_actor (cast `/Game/Blueprints/Daniel/RandomObjectsRoom/ReplaceableMeshActor` _array_element))
      (`/Game/Blueprints/Daniel/RandomObjectsRoom/ReplaceableMeshActor.MoveMesh` _asreplaceable_mesh_actor (`KismetMathLibrary.MakeVector` (.x (`self.K2_GetActorLocation`)) (.y (`self.K2_GetActorLocation`)) 5.0) 6))))

(event `MoveLeftCollider`
  ;[1 1 1] Decide Direction For Left Door
  (switch `int` (`self.Ldir`)
    (:`0`
      (`self.RepLBlock` (* (`self.GetActorRightVector`) -30)))
    (:`1`
      (`self.RepLBlock` (* (`self.GetActorRightVector`) 30)))))

(event `OpenLeftDoor`
  (bind _lrotcount (`self.LRotCount`))
  (bind _lrotcount_2 (`self.LRotCount`))
  (bind _lrotcount_3 (`self.LRotCount`))
  (bind _lrotcount_4 (`self.LRotCount`))
  ;[1 1 1] Swing Doors
  (bind _ashider (cast `/Game/HiderBP/Blueprints/Hider` (`self.Player`))
    (:`then`
      (if (`/Game/HiderBP/Blueprints/Hider.IsFlash` _ashider)
        (switch `int` (`self.Ldir`)
          (:`0`
            (if (not (< _lrotcount_3 -90.0))
              (`self.RepLRot` (struct :`Yaw` -10.0))
              (set `self.LRotCount` (- _lrotcount_3 10.0))))
          (:`1`
            (if (not (> _lrotcount_4 90.0))
              (`self.RepLRot` (struct :`Yaw` 10.0))
              (set `self.LRotCount` (+ _lrotcount_4 10.0)))))
        (else
          (switch `int` (`self.Ldir`) :!label _label
            (:`0`
              (if (not (< _lrotcount -90.0))
                (`self.RepLRot` (struct :`Yaw` -5.0))
                (set `self.LRotCount` (- _lrotcount 5.0))))
            (:`1`
              (if (not (> _lrotcount_2 90.0))
                (`self.RepLRot` (struct :`Yaw` 5.0))
                (set `self.LRotCount` (+ _lrotcount_2 5.0))))))))
    (:`CastFailed`
      (goto _label))))

(event `self.ReceiveTick`
  (params (DeltaSeconds :type "Float (single-precision)"))
  ;[1 1 1] Swing Doors
  (`/Engine/EditorBlueprintResources/ActorMacros.Switch Has Authority`
    (:`Authority`
      (`|ExecutionSequence`
        (:`then_0`
          (`self.SwingLeftDoor`))
        (:`then_1`
          (`self.SwingRightDoor`))
        (:`then_2`
          (`self.CheckSpace`))
        (:`then_3`
          (`self.ResetDoor`))))))

(event `ResetLeftDoor`
  (bind _lrotcount (`self.LRotCount`))
  ;[1 1 1] Reset Door
  (if (> _lrotcount 0.0)
    (`self.RepLRot` (struct :`Yaw` -3.0))
    (set `self.LRotCount` (- _lrotcount 3.0))
    (else
      (`self.RepLRot` (struct :`Yaw` 3.0))
      (set `self.LRotCount` (+ (`self.LRotCount`) 3.0)))))

(event `ResetDoor`
  ;[1 1 1] Reset Door
  (`/Engine/EditorBlueprintResources/ActorMacros.Switch Has Authority`
    (:`Authority`
      (`|ExecutionSequence`
        (:`then_0`
          (if (`self.HitLeft`)
            _
            (elif (!= (`self.LRotCount`) 0.0)
              (`self.ResetLeftDoor`))))
        (:`then_1`
          (if (`self.HitRight`)
            _
            (elif (!= (`self.RRotCount`) 0.0)
              (`self.ResetRightDoor`))))))))

(event `OpenRightDoor`
  (bind _rrotcount (`self.RRotCount`))
  (bind _rrotcount_2 (`self.RRotCount`))
  (bind _rrotcount_3 (`self.RRotCount`))
  (bind _rrotcount_4 (`self.RRotCount`))
  ;[1 1 1] Swing Doors
  (bind _ashider (cast `/Game/HiderBP/Blueprints/Hider` (`self.Player`))
    (:`then`
      (if (`/Game/HiderBP/Blueprints/Hider.IsFlash` _ashider)
        (switch `int` (`self.Rdir`)
          (:`0`
            (if (not (< _rrotcount_4 -90.0))
              (`self.RepRRot` (struct :`Yaw` 10.0))
              (set `self.RRotCount` (- _rrotcount_4 10.0))))
          (:`1`
            (if (not (> _rrotcount_3 90.0))
              (`self.RepRRot` (struct :`Yaw` -10.0))
              (set `self.RRotCount` (+ _rrotcount_3 10.0)))))
        (else
          (switch `int` (`self.Rdir`) :!label _label_2
            (:`0`
              (if (not (< _rrotcount_2 -90.0))
                (`self.RepRRot` (struct :`Yaw` 5.0))
                (set `self.RRotCount` (- _rrotcount_2 5.0))))
            (:`1`
              (if (not (> _rrotcount 90.0))
                (`self.RepRRot` (struct :`Yaw` -5.0))
                (set `self.RRotCount` (+ _rrotcount 5.0))))))))
    (:`CastFailed`
      (goto _label_2))))

(event `ResetRightDoor`
  (bind _rrotcount (`self.RRotCount`))
  ;[1 1 1] Reset Door
  (if (> _rrotcount 0.0)
    (`self.RepRRot` (struct :`Yaw` 3.0))
    (set `self.RRotCount` (- _rrotcount 3.0))
    (else
      (`self.RepRRot` (struct :`Yaw` -3.0))
      (set `self.RRotCount` (+ (`self.RRotCount`) 3.0)))))

(fn `CalculateSwingingDir`
  (params (PlayerPos :type "Vector Structure"))
  (returns (Dir :type Integer))
  (if (> (`KismetMathLibrary.Dot_VectorVector` (- PlayerPos (`self.K2_GetActorLocation`)) (`self.GetActorRightVector`)) 0.0)
    (return 0)
    (else
      (return 1))))

(fn `CheckParallelVelocity`
  (returns (IsPerpendicular :type Boolean))
  (return (== (`KismetMathLibrary.Dot_VectorVector` (`self.GetVelocity` (`self.Player`)) (`self.GetActorRightVector`)) 0.0)))

(fn `CheckVelocityDir`
  (returns (SameVelDir :type Boolean))
  (bind _initveldir (`self.InitVelDir`))
  (if (> (`KismetMathLibrary.Dot_VectorVector` (`self.GetVelocity` (`self.Player`)) (`self.GetActorRightVector`)) 0.0)
    (bind _output_get (set `self.VelDir` 1))
    (return (== _output_get _initveldir))
    (else
      (bind _output_get_2 (set `self.VelDir` 0))
      (return (== _initveldir _output_get_2)))))

(fn `SetVelocityDir`
  (if (> (`KismetMathLibrary.Dot_VectorVector` (`self.GetVelocity` (`self.Player`)) (`self.GetActorRightVector`)) 0.0)
    (set `self.InitVelDir` 1)
    (else
      (set `self.InitVelDir` 0))))

(fn `SwingLeftDoor`
  (if (`self.HitLeft`)
    (if (> (`KismetMathLibrary.VSize` (`self.GetVelocity` (`self.Player`))) 0.0)
      (bind _isperpendicular (`self.CheckParallelVelocity`))
      (if (not _isperpendicular)
        (bind _sameveldir (`self.CheckVelocityDir`))
        (if _sameveldir
          (`self.OpenLeftDoor`))))))

(fn `SwingRightDoor`
  (if (`self.HitRight`)
    (if (> (`KismetMathLibrary.VSize` (`self.GetVelocity` (`self.Player`))) 0.0)
      (bind _isperpendicular (`self.CheckParallelVelocity`))
      (if (not _isperpendicular)
        (bind _sameveldir (`self.CheckVelocityDir`))
        (if _sameveldir
          (`self.OpenRightDoor`))))))

(fn `UserConstructionScript`)