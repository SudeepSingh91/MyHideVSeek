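; Objective marker Blueprint that feeds the active target area to the local player's HUD as an objective message while that player controls a Hider.
; BeginPlay caches the first TargetAreasManager found in the level.
; Tick polls the local player stored on CTPGameState, checks the pawn is a Hider, and calls SetObjectiveMessage whenever the manager's ActiveArea is valid.
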(event `self.ReceiveBeginPlay`
  (bind _outactors (`GameplayStatics.GetAllActorsOfClass` "/Game/Blueprints/Daniel/CTP/TargetAreasManager.TargetAreasManager_C"))
  (set `self.AreasManager` (`KismetArrayLibrary.Array_Get` _outactors)))

(event `self.ReceiveTick`
  (params (DeltaSeconds :type "Float (single-precision)"))
  (bind _activearea (`/Game/Blueprints/Daniel/CTP/TargetAreasManager.ActiveArea` (`self.AreasManager`)))
  (bind _asctpgame_state (cast `/Game/Blueprints/Daniel/CTP/CTPGameState` (`GameplayStatics.GetGameState`)))
  (bind _localplayer (`/Game/Blueprints/Daniel/CTP/CTPGameState.LocalPlayer` _asctpgame_state))
  (cast `/Game/HiderBP/Blueprints/Hider` (`Controller.K2_GetPawn` _localplayer))
  (if (`KismetSystemLibrary.IsValid` _activearea)
    (message `/Game/Blueprints/Arpit/ObjectiveMarker_Interface.SetObjective` (`PlayerController.GetHUD` _localplayer) (`|MakeArray` _activearea :!type "Actor Object Reference"))))

(fn `UserConstructionScript`)