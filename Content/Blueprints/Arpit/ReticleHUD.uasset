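; HUD Blueprint that draws the aiming reticle and on-screen objective markers.
; Each DrawHUD draws the reticle texture near screen center, shifted by offset variables.
; For each actor in CurrentObjective, it projects the location to screen and, if in front of the camera, draws a material icon and label with distance in meters from the player pawn.
; SetObjective replaces the tracked objective list.
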(event `self.ReceiveDrawHUD`
  (params (SizeX :type Integer) (SizeY :type Integer))
  (`|ExecutionSequence`
    (:`then_0`
      (`self.DrawTextureSimple` self (`self.ReticleTxt`) (+ (- (`KismetMathLibrary.Conv_IntToDouble` (/ SizeX 2)) 69.0) (`self.ScrXDiff`)) (+ (- (`KismetMathLibrary.Conv_IntToDouble` (/ SizeY 2)) 61.0) (`self.ScrYDiff`)) 0.75 false))
    (:`then_1`
      (for _array_element (`self.Current_Objective`)
        (bind _returnvalue (`self.K2_GetActorLocation` _array_element))
        (bind _y (.y (`self.Project` _returnvalue)))
        (if (> (.z (`self.Project` _returnvalue)) 0.0)
          (bind _returnvalue_2 (`KismetStringLibrary.Concat_StrStr` "Objective :" (`KismetStringLibrary.Conv_IntToString` (`KismetMathLibrary.Round` (/ (`KismetMathLibrary.VSize` (- (`self.K2_GetActorLocation` (`GameplayStatics.GetPlayerPawn` 0)) _returnvalue)) 100.0))) "m"))
          (bind _returnvalue_3 (- (.x (`self.Project` _returnvalue)) (/ (`self.GetTextSize` _returnvalue_2 "/Engine/EngineFonts/RobotoDistanceField.RobotoDistanceField") 2.0)))
          (`self.DrawText` _returnvalue_2 (struct :`R` 1.0 :`G` 1.0 :`B` 1.0 :`A` 1.0) (+ _returnvalue_3 20.0) (- _y 100.0) "/Engine/EngineFonts/RobotoDistanceField.RobotoDistanceField" 0.5)
          (`self.DrawMaterialSimple` "/Game/Blueprints/Arpit/Test_Asset/Objective_Material.Objective_Material" (+ _returnvalue_3 50.0) (- _y 85.0) 256.0 256.0 0.175))))))

(event `/Game/Blueprints/Arpit/ObjectiveMarker_Interface.SetObjective`
  (params (Objective :type "Array of Actor Object Reference (by ref)"))
  (set `self.Current_Objective` Objective))

(fn `UserConstructionScript`)