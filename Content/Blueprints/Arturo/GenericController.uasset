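; GenericController is a player controller for the front-end menus, switching between a start menu and a selection menu.
; Two seconds after BeginPlay, the authority side calls ClientHUD, which creates both widgets, sets UI-only input and hides the selection menu.
; Events toggle the menus' visibility, and HostGame passes the controller to SelectionInstance's host function.
; JoinGame and ExitGame are empty stubs.
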(event `self.ReceiveBeginPlay`
  (`KismetSystemLibrary.Delay` 2.0)
  (`/Engine/EditorBlueprintResources/ActorMacros.Switch Has Authority`
    (:`Authority`
      (`self.ClientHUD`))))

(event `ClientHUD`
  (bind _returnvalue (`|CreateWidget` "/Game/Blueprints/Arturo/Widgets/StartMenu.StartMenu_C" self))
  (bind _output_get (set `self.StartMenu` _returnvalue))
  (`UserWidget.AddToViewport` _output_get 0)
  (`WidgetBlueprintLibrary.SetInputMode_UIOnlyEx` self _output_get)
  (bind _returnvalue_2 (`|CreateWidget` "/Game/Blueprints/Arturo/Widgets/SelectMenu.SelectMenu_C" self))
  (bind _output_get_2 (set `self.SelectMenu` _returnvalue_2))
  (`UserWidget.AddToViewport` _output_get_2 0)
  (`WidgetBlueprintLibrary.SetInputMode_UIOnlyEx` self _output_get_2)
  (`Widget.SetVisibility` (`self.SelectMenu`) "Hidden"))

(event `HostGame`
  (bind _asselection_instance (cast `/Game/Blueprints/Arturo/SelectionInstance` (`GameplayStatics.GetGameInstance`)))
  (`/Game/Blueprints/Arturo/SelectionInstance.SelectionInst_Host` _asselection_instance self))

(event `JoinGame`)

(event `ExitGame`)

(event `Start-Select`
  (`Widget.SetVisibility` (`self.StartMenu`) "Hidden")
  (`Widget.SetVisibility` (`self.SelectMenu`) "Visible"))

(event `Select-Start`
  (`Widget.SetVisibility` (`self.SelectMenu`) "Hidden")
  (`Widget.SetVisibility` (`self.StartMenu`) "Visible"))

(fn `UserConstructionScript`)