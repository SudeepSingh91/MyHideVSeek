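; Projectile that damages Hiders on overlap, with hit logic running only on the server.
; Trigger boxes and ReplaceableMeshActors set a hit flag and destroy it, blocking later hits on players.
; An unblocked hit deals damage to a Hider and destroys the projectile, or calls ChangeToHider on a Hider_Practice without destroying it.
; Mesh rotation and water-mesh swap events exist, but their calls here are disconnected.
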(event `setRotation`
  (`SceneComponent.K2_AddWorldRotation` (`self.StaticMeshComponent`) (struct :`Yaw` 90.0) false false))

(event `SetWaterMesh`
  (bind _item (`KismetArrayLibrary.Array_Get` (`self.WaterMesh`) (`self.ArrIter`)))
  (`StaticMeshComponent.SetStaticMesh` (`self.StaticMeshComponent`) _item)
  (`KismetSystemLibrary.PrintString` (`KismetSystemLibrary.GetDisplayName` _item)))

(event `self.ReceiveBeginPlay`
  (`/Engine/EditorBlueprintResources/ActorMacros.Switch Has Authority`))

(event `self.StaticMeshComponent.OnComponentBeginOverlap`
  (params (OverlappedComponent :type "PrimitiveComponent Object Reference") (OtherActor :type "Actor Object Reference") (OtherComp :type "PrimitiveComponent Object Reference") (OtherBodyIndex :type Integer) (bFromSweep :type Boolean) (SweepResult :type "HitResult Structure (by ref)"))
  ;[1 1 1] Damaged The Hider
  (`/Engine/EditorBlueprintResources/ActorMacros.Switch Has Authority`
    (:`Authority`
      (cast `TriggerBox` OtherActor
        (:`then`
          (set `self.DidHit` true)
          (`self.K2_DestroyActor`))
        (:`CastFailed`
          (cast `/Game/Blueprints/Daniel/RandomObjectsRoom/ReplaceableMeshActor` OtherActor
            (:`then`
              (set `self.DidHit` true)
              (`self.K2_DestroyActor`))
            (:`CastFailed`
              (bind _ashider (cast `/Game/HiderBP/Blueprints/Hider` OtherActor)
                (:`then`
                  (if (not (`self.DidHit`))
                    (`/Game/HiderBP/Blueprints/Hider.ReceiveDamage` _ashider 1)
                    (`self.K2_DestroyActor`)))
                (:`CastFailed`
                  (bind _ashider_practice (cast `/Game/Blueprints/Sudeep/Hider_Practice` OtherActor))
                  (if (not (`self.DidHit`))
                    (`/Game/Blueprints/Sudeep/Hider_Practice.Change to Hider` _ashider_practice)))))))))))

(fn `UserConstructionScript`)